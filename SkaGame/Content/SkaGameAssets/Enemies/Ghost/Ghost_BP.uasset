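; Ghost enemy for a side-scroller that roams, chases the player and melee attacks, driven by a simple AIState machine.
; CheckState dispatches to random navmesh roaming, AIMoveTo chase or montage attack; PawnSensing triggers the chase, and reaching the player triggers the attack.
; A finger-socket sphere damages the player on overlap, with collision toggled by DamageAllowed and DamageNotAllowed events.
; Incoming damage plays a hurt montage and destroys the ghost when health runs out.
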(event `Roam`
  ;[1 1 1] Roam
  (if (not (`self.isAttacking?`))
    (`|AIMoveTo` self (`NavigationSystem.GetRandomPointInNavigableRadius` (`self.K2_GetActorLocation`) 500.0) null 10.0
      (:`OnSuccess`
        _)
      (:`OnFail`
        _))
    (`KismetSystemLibrary.Delay` 0.5)
    (`self.CheckState`)))

(event `self.ReceiveBeginPlay`
  ;[1 1 1] Initialize Ghost
  (`PrimitiveComponent.SetCollisionEnabled` (`self.AttackCollisionSphere`) "NoCollision")
  (set `self.AIState` "NewEnumerator1")
  (`self.CheckState`))

(event `CheckState`
  ;[1 1 1] Checks the state of the AI Tree
  (switch `/Game/SkaGameAssets/Enemies/DarnBat/BluePrints/E_AI_State` (`self.AIState`)
    (:`NewEnumerator1`
      (`self.Roam`))
    (:`NewEnumerator2`
      (`self.ChasePlayer` (`GameplayStatics.GetPlayerPawn` 0)))
    (:`NewEnumerator3`
      (`self.Attack`))))

(event `ChasePlayer`
  (params (PlayertoChase :type "Pawn Object Reference"))
  ;[1 1 1] Chases player
  (if (not (`self.isAttacking?`))
    (`|AIMoveTo` self (0.0 0.0 0.0) PlayertoChase 10.0
      (:`OnSuccess`
        (set `self.AIState` "NewEnumerator3")
        (`self.CheckState`)))))

(event `self.ReceiveAnyDamage`
  (params (Damage :type "Float (single-precision)") (DamageType :type "DamageType Object Reference") (InstigatedBy :type "Controller Object Reference") (DamageCauser :type "Actor Object Reference"))
  ;[1 1 1] Ghost Damage
  (set `self.Health` (- (`self.Health`) Damage))
  (`AnimInstance.Montage_Play` (`SkeletalMeshComponent.GetAnimInstance` (`self.Mesh`)) "/Game/SkaGameAssets/Enemies/Ghost/GhostHurn_Montage.GhostHurn_Montage" 1.0 "MontageLength" 0.0)
  (`self.CheckForDeath`))

(event `self.PawnSensing.OnSeePawn`
  (params (Pawn :type "Pawn Object Reference"))
  ;[1 1 1] Sets AI state when it senses playe pawn
  (set `self.AIState` "NewEnumerator2")
  (bind _asside_scroller_character (cast `/Game/SkaGameAssets/Brad/Blueprints/SideScrollerCharacter` Pawn))
  (`self.ChasePlayer` _asside_scroller_character))

(event `CheckForDeath`
  ;[1 1 1] Check for death
  (if (<= (`self.Health`) 0.0)
    (`self.K2_DestroyActor`)))

(event `Attack`
  ;[1 1 1] Attack
  (set `self.isAttacking?` true)
  (`AnimInstance.Montage_Play` (`SkeletalMeshComponent.GetAnimInstance` (`self.Mesh`)) "/Game/SkaGameAssets/Enemies/Ghost/GhostAttack_Montage.GhostAttack_Montage" 1.0 "MontageLength" 0.0)
  (`KismetSystemLibrary.Delay` 0.5)
  (set `self.AIState` "NewEnumerator2")
  (set `self.isAttacking?` false)
  (`self.CheckState`))

(event `DamageNotAllowed`
  ;[1 1 1] Attack
  ;;[1 1 1] Damage Handling
  (`PrimitiveComponent.SetCollisionEnabled` (`self.AttackCollisionSphere`) "NoCollision"))

(event `DamageAllowed`
  ;[1 1 1] Attack
  ;;[1 1 1] Damage Handling
  (`PrimitiveComponent.SetCollisionEnabled` (`self.AttackCollisionSphere`) "QueryOnly"))

(event `self.AttackCollisionSphere.OnComponentBeginOverlap`
  (params (OverlappedComponent :type "PrimitiveComponent Object Reference") (OtherActor :type "Actor Object Reference") (OtherComp :type "PrimitiveComponent Object Reference") (OtherBodyIndex :type Integer) (bFromSweep :type Boolean) (SweepResult :type "HitResult Structure (by ref)"))
  ;[1 1 1] Attack
  ;;[1 1 1] Damage Handling
  (bind _asside_scroller_character (cast `/Game/SkaGameAssets/Brad/Blueprints/SideScrollerCharacter` OtherActor))
  (`GameplayStatics.ApplyDamage` _asside_scroller_character 0.1)
  (`KismetSystemLibrary.PrintString` "Brad Got Slammed!!!!")
  (`KismetSystemLibrary.Delay` 0.4))

(fn `UserConstructionScript`
  (`SceneComponent.K2_AttachToComponent` (`self.AttackCollisionSphere`) (`self.Mesh`) "Finger_L_end" "KeepRelative" "KeepRelative" "KeepRelative" true))