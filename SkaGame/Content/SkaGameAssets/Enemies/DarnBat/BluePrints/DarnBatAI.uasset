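; DarnBatAI is the AI controller for the DarnBat enemy, walking it along a linked chain of nodes.
; On BeginPlay it stores the controlled DarnBat pawn and moves toward that pawn's DesiredNode.
; Each Tick, when move status differs from DesiredStatus, it advances DesiredNode to its NextNode.
; It then moves to the node after the new DesiredNode, so the target runs one link ahead.
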(event `self.ReceiveBeginPlay`
  (bind _asdarn_bat_character_bp (cast `/Game/SkaGameAssets/Enemies/DarnBat/BluePrints/DarnBat_CharacterBP` (`self.K2_GetPawn`)))
  (bind _output_get (set `self.Storedpawn` _asdarn_bat_character_bp))
  (`self.MoveToActor` (`/Game/SkaGameAssets/Enemies/DarnBat/BluePrints/DarnBat_CharacterBP.DesiredNode` _output_get) 15.0))

(event `self.ReceiveTick`
  (params (DeltaSeconds :type "Float (single-precision)"))
  (bind _storedpawn (`self.Storedpawn`))
  (bind _nextnode (`/Game/SkaGameAssets/Enemies/DarnBat/BluePrints/PathNode.NextNode` (`/Game/SkaGameAssets/Enemies/DarnBat/BluePrints/DarnBat_CharacterBP.DesiredNode` _storedpawn)))
  (if (`|EnumInequality` (`self.GetMoveStatus`) (`self.DesiredStatus`))
    (set `/Game/SkaGameAssets/Enemies/DarnBat/BluePrints/DarnBat_CharacterBP.DesiredNode` _nextnode _storedpawn)
    (`self.MoveToActor` _nextnode 15.0)))

(fn `UserConstructionScript`)