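; DarnBat enemy character that either roams or chases the player, and destroys itself when its Health runs out.
; AIState picks the starting behavior on BeginPlay: Roam repeatedly moves to random nearby navigable points.
; Pawn sensing calls ChasePlayer on a seen SideScrollerCharacter without updating AIState.
; ChasePlayer re-calls itself after each successful move but passes no target, and Tick polls Health for death.
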(event `self.ReceiveBeginPlay`
  (switch `/Game/SkaGameAssets/Enemies/DarnBat/BluePrints/E_AI_State` (`self.AIState`)
    (:`NewEnumerator1`
      (`self.Roam`))
    (:`NewEnumerator2`
      (`self.ChasePlayer` null))))

(event `Roam`
  ;[1 1 1] Roam
  (`|AIMoveTo` self (`NavigationSystem.GetRandomPointInNavigableRadius` (`self.K2_GetActorLocation`) 500.0)
    (:`then`
      (`KismetSystemLibrary.Delay` 1.0)
      (`self.Roam`))))

(event `ChasePlayer`
  (params (PlayertoChase :type "Pawn Object Reference"))
  ;[1 1 1] ChasePlayer
  (`|AIMoveTo` self (0.0 0.0 0.0) PlayertoChase
    (:`OnSuccess`
      (`KismetSystemLibrary.Delay` 1.0)
      (`self.ChasePlayer` null))))

(event `self.ReceiveTick`
  (params (DeltaSeconds :type "Float (single-precision)"))
  ;[1 1 1] health/damage
  (if (<= (`self.Health`) 0.0)
    (`self.K2_DestroyActor`)))

(event `self.PawnSensing.OnSeePawn`
  (params (Pawn :type "Pawn Object Reference"))
  ;[1 1 1] chase player when we see the them
  (bind _asside_scroller_character (cast `/Game/SkaGameAssets/Brad/Blueprints/SideScrollerCharacter` Pawn))
  (`self.ChasePlayer` _asside_scroller_character))

(fn `UserConstructionScript`)