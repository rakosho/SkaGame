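; Ghost enemy for a side-scroller that spawns a right-side barrier on BeginPlay and removes it on death.
; Damage reduces health and plays a hurt-montage stun that blocks further damage and attacks.
; AttackPlayer plays a gated montage; a finger-socket sphere, toggled by DamageAllowed/DamageNotAllowed, damages the player on overlap.
; An AIState switch runs every Tick, but Roam and Chase are empty, their movement logic disconnected.
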(event `self.ReceiveBeginPlay`
  ;[1 1 1] Initialize Ghost
  (`|ExecutionSequence`
    (:`then_0`
      (`PrimitiveComponent.SetCollisionEnabled` (`self.AttackCollisionSphere`) "NoCollision")
      (set `self.AIState` "NewEnumerator1")
      (`self.CheckState`))
    (:`then_1`
      (`|ExecutionSequence`
        (:`then_1`
          (bind _returnvalue (`|SpawnActorFromClass` "/Game/SkaGameAssets/BluePrints/right_Barrier.right_Barrier_C" (`KismetMathLibrary.Conv_VectorToTransform` (+ (`self.K2_GetActorLocation`) (0.0 -1000.0 0.0))) "Undefined" "OverrideRootScale")))))))

(event `CheckForDeath`
  ;[1 1 1] Check for death
  (if (<= (`self.Health`) 0.0)
    (`|ExecutionSequence`
      (:`then_0`
        (`self.K2_DestroyActor`))
      (:`then_2`
        (`/Game/SkaGameAssets/BluePrints/right_Barrier.destroyRight` (stale `self.ReceiveBeginPlay` _returnvalue))))))

(event `CheckState`
  ;[1 1 1] Checks the state of the AI Tree
  (switch `/Game/SkaGameAssets/Enemies/GhostAssests/AI/Ghost_AI_State` (`self.AIState`) :!label _label
    (:`NewEnumerator1`
      (`self.Roam`))
    (:`NewEnumerator2`
      (`self.ChasePlayer` (`GameplayStatics.GetPlayerPawn` 0)))
    (:`NewEnumerator3`
      (`self.Attack`))))

(event `Stun`
  ;[1 1 1] Stun
  (set `self.isStunned?` true)
  (bind _returnvalue (`AnimInstance.Montage_Play` (`SkeletalMeshComponent.GetAnimInstance` (`self.Mesh`)) "/Game/SkaGameAssets/Enemies/GhostAssests/Animations/GhostHurn_Montage.GhostHurn_Montage" 1.25 "MontageLength" 0.0))
  (`KismetSystemLibrary.Delay` _returnvalue)
  (set `self.isStunned?` false))

(event `self.ReceiveTick`
  (params (DeltaSeconds :type "Float (single-precision)"))
  ;[1 1 1] Checks the state of the AI Tree
  (goto _label))

(event `Roam`
  ;[1 1 1] Deprecated Cpde
  ;;[1 1 1] Roam
)

(event `/Game/SkaGameAssets/Enemies/GhostAssests/AI/HealthInterFace.AttackPlayer`
  ;[1 1 1] Attack
  (if (not (`self.isStunned?`))
    (set `self.isAttacking?` true)
    (`/Engine/EditorBlueprintResources/StandardMacros.DoOnce` false :!label _label_2
      (:`Completed`
        (bind _returnvalue (`AnimInstance.Montage_Play` (`SkeletalMeshComponent.GetAnimInstance` (`self.Mesh`)) "/Game/SkaGameAssets/Enemies/GhostAssests/Animations/GhostAttack_Montage.GhostAttack_Montage" 1.0 "MontageLength" 0.0))
        (`KismetSystemLibrary.Delay` _returnvalue)
        (goto _label_2 :!via `Reset`)))))

(event `self.ReceiveAnyDamage`
  (params (Damage :type "Float (single-precision)") (DamageType :type "DamageType Object Reference") (InstigatedBy :type "Controller Object Reference") (DamageCauser :type "Actor Object Reference"))
  ;[1 1 1] HealthHandling
  (if (not (`self.isStunned?`))
    (`self.Stun`)
    (set `self.Health` (- (`self.Health`) Damage))
    (`self.CheckForDeath`)))

(event `ChasePlayer`
  (params (PlayertoChase :type "Pawn Object Reference"))
  ;[1 1 1] Deprecated Cpde
  ;;[1 1 1] Chases player
)

(event `DamageAllowed`
  ;[1 1 1] Attack
  ;;[1 1 1] Damage Handling
  (`PrimitiveComponent.SetCollisionEnabled` (`self.AttackCollisionSphere`) "QueryOnly"))

(event `DamageNotAllowed`
  ;[1 1 1] Attack
  ;;[1 1 1] Damage Handling
  (`PrimitiveComponent.SetCollisionEnabled` (`self.AttackCollisionSphere`) "NoCollision"))

(event `self.AttackCollisionSphere.OnComponentBeginOverlap`
  (params (OverlappedComponent :type "PrimitiveComponent Object Reference") (OtherActor :type "Actor Object Reference") (OtherComp :type "PrimitiveComponent Object Reference") (OtherBodyIndex :type Integer) (bFromSweep :type Boolean) (SweepResult :type "HitResult Structure (by ref)"))
  ;[1 1 1] Attack
  ;;[1 1 1] Damage Handling
  (if (not (`self.isStunned?`))
    (bind _asside_scroller_character (cast `/Game/SkaGameAssets/Brad/Blueprints/SideScrollerCharacter` OtherActor))
    (`GameplayStatics.ApplyDamage` _asside_scroller_character 0.1)
    (`KismetSystemLibrary.PrintString` "Brad Got Slammed!!!!")
    (`KismetSystemLibrary.Delay` 0.4)))

(fn `UserConstructionScript`
  (`SceneComponent.K2_AttachToComponent` (`self.AttackCollisionSphere`) (`self.Mesh`) "Finger_L_end" "KeepRelative" "KeepRelative" "KeepRelative" true))