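; PilPol enemy Blueprint for a Polgergust character with a "HealthNab" grab attack and simple health.
; AttackPlayer enables a hit sphere socketed to the right middle finger and plays a DoOnce-gated montage, then a success or fail montage.
; Sphere overlap deals damage and flags success.
; Incoming damage reduces health unless briefly stunned, destroying the actor at zero; barrier and AI-state logic is left disconnected.
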(event `self.ReceiveBeginPlay`
  ;[1 1 1] Initialize PilPol
  (`PrimitiveComponent.IgnoreActorWhenMoving` (`self.Sphere`) self true))

(event `CheckForDeath`
  ;[1 1 1] Check for death
  (if (<= (`self.Health`) 0.0)
    (`self.K2_DestroyActor`)))

(event `self.ReceiveAnyDamage`
  (params (Damage :type "Float (single-precision)") (DamageType :type "DamageType Object Reference") (InstigatedBy :type "Controller Object Reference") (DamageCauser :type "Actor Object Reference"))
  ;[1 1 1] Health Management
  (if (not (`self.isStunned?`))
    (`self.Stun`)
    (set `self.Health` (- (`self.Health`) Damage))
    (`self.CheckForDeath`)))

(event `Stun`
  ;[1 1 1] Stun
  (set `self.isStunned?` true)
  (`AnimInstance.Montage_Play` (`SkeletalMeshComponent.GetAnimInstance` (`self.Mesh`)) "/Game/SkaGameAssets/Enemies/PilPolAssests/Animations/PilPol_Anim_Polgergust_Armature_Polgergust_Hurt_Montage.PilPol_Anim_Polgergust_Armature_Polgergust_Hurt_Montage" 1.0 "MontageLength" 0.0)
  (`KismetSystemLibrary.Delay` 0.2)
  (set `self.isStunned?` false))

(event `/Game/SkaGameAssets/Enemies/GhostAssests/AI/HealthInterFace.AttackPlayer`
  (bind _returnvalue (`SkeletalMeshComponent.GetAnimInstance` (`self.Mesh`)))
  ;[1 1 1] HealthNab
  (`PrimitiveComponent.SetCollisionEnabled` (`self.Sphere`) "QueryAndPhysics")
  (`/Engine/EditorBlueprintResources/StandardMacros.DoOnce` false :!label _label
    (:`Completed`
      (bind _returnvalue_2 (`AnimInstance.Montage_Play` _returnvalue "/Game/SkaGameAssets/Enemies/PilPolAssests/Animations/PilPol_Anim_Polgergust_Armature_Polgergust_HealthNab_Montage.PilPol_Anim_Polgergust_Armature_Polgergust_HealthNab_Montage" 1.0 "MontageLength" 0.0))
      (`KismetSystemLibrary.Delay` _returnvalue_2)
      (if (`self.HealthNabSucceeded?`)
        (`AnimInstance.Montage_Play` _returnvalue "/Game/SkaGameAssets/Enemies/PilPolAssests/Animations/PilPol_Anim_Polgergust_Armature_Polgergust_HealthNab_Success_Montage.PilPol_Anim_Polgergust_Armature_Polgergust_HealthNab_Success_Montage" 0.5 "MontageLength" 0.0)
        (set `self.HealthNabSucceeded?` false)
        (`KismetSystemLibrary.Delay` 2.0)
        (goto _label :!via `Reset`)
        (else
          (bind _returnvalue_3 (`AnimInstance.Montage_Play` _returnvalue "/Game/SkaGameAssets/Enemies/PilPolAssests/Animations/PilPol_Anim_Polgergust_Armature_Polgergust_HealthNab_Fail_Montage.PilPol_Anim_Polgergust_Armature_Polgergust_HealthNab_Fail_Montage" 1.0 "MontageLength" 0.0))
          (`KismetSystemLibrary.Delay` _returnvalue_3)
          (goto _label :!via `Reset`))))))

(event `self.Sphere.OnComponentBeginOverlap`
  (params (OverlappedComponent :type "PrimitiveComponent Object Reference") (OtherActor :type "Actor Object Reference") (OtherComp :type "PrimitiveComponent Object Reference") (OtherBodyIndex :type Integer) (bFromSweep :type Boolean) (SweepResult :type "HitResult Structure (by ref)"))
  ;[1 1 1] HealthNab
  (set `self.HealthNabSucceeded?` true)
  (`GameplayStatics.ApplyDamage` OtherActor 0.1))

(fn `UserConstructionScript`
  (`SceneComponent.K2_AttachToComponent` (`self.Sphere`) (`self.Mesh`) "Finger_Middle_R" "SnapToTarget" "SnapToTarget" "KeepRelative" true))