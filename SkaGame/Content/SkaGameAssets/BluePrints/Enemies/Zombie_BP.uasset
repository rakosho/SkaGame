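; Zombie enemy that lies inactive until it first sees a pawn, then chases and attacks in melee.
; An AIState enum drives CheckState, cycling between roam, AI MoveTo chase and montage attack.
; A sphere on the right-hand socket deals overlap damage, with functions to toggle its collision.
; Incoming damage causes flinches, a temporary invulnerable knockdown every third hit, and delayed destruction at zero health.
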(event `Check Down`
  ;[1 1 1] CHeck if Down
  (if (== (`self.KnockDownCount`) 3)
    (set `self.Is Down?` true)
    (`KismetSystemLibrary.Delay` 3.0)
    (set `self.KnockDownCount` 0)
    (set `self.Is Down?` false)
    (`self.Check State`)
    (else
      (`AnimInstance.Montage_Play` (`SkeletalMeshComponent.GetAnimInstance` (`self.Mesh`)) "/Game/SkaGameAssets/Enemies/Zombie_Anim_Zombie_Armature_Zombie_Flinch_Montage.Zombie_Anim_Zombie_Armature_Zombie_Flinch_Montage" 1.0 "MontageLength" 0.0)
      (`KismetSystemLibrary.Delay` 0.2))))

(event `Wait`
  ;[1 1 1] Wait
  (`KismetSystemLibrary.Delay` 1.5)
  (`self.K2_DestroyActor`))

(event `/Game/SkaGameAssets/BluePrints/Enemies/AI/HealthInterFace.HealthInterFaceDamage`
  (params (Damage :type "Float (single-precision)"))
  ;[1 1 1] Health Damage
  (`KismetSystemLibrary.PrintString` "zombie got slammed")
  (if (not (`self.Is Down?`))
    (set `self.Health` (- (`self.Health`) Damage))
    (`/Engine/EditorBlueprintResources/StandardMacros.IncrementInt` (`self.KnockDownCount`)
      (:`  `
        (`self.Check Down`)
        (`self.CheckDeath`)))))

(event `self.ReceiveAnyDamage`
  (params (Damage :type "Float (single-precision)") (DamageType :type "DamageType Object Reference") (InstigatedBy :type "Controller Object Reference") (DamageCauser :type "Actor Object Reference"))
  ;[1 1 1] Health Damage
  (`KismetSystemLibrary.Delay` 0.2)
  (`self.HealthInterFaceDamage` Damage))

(event `self.ReceiveBeginPlay`
  (set `self.Is Down?` true)
  (`PrimitiveComponent.IgnoreComponentWhenMoving` (`self.Sphere`) (`self.CapsuleComponent`) true)
  (`self.Check State`))

(event `Chase Player`
  (params (`Player To chase` :type "Pawn Object Reference"))
  ;[1 1 1] Chase Player
  (if (`self.Is Down?`)
    _
    (elif (not (`self.Is Stunned?`))
      (`|AIMoveTo` self (0.0 0.0 0.0) `Player To chase` 5.0
        (:`OnSuccess`
          (set `self.AI State` "NewEnumerator3"))
        (:`OnFail`
          _))
      (`KismetSystemLibrary.Delay` 0.1)
      (`self.Check State`))))

(event `Roam`
  ;[1 1 1] Roam
  (if (`self.Is Down?`)
    _
    (elif (not (`self.Is Attacking?`))
      (`|AIMoveTo` self (`NavigationSystem.GetRandomPointInNavigableRadius` (`self.K2_GetActorLocation`) 500.0) null 10.0
        (:`OnSuccess`
          _)
        (:`OnFail`
          _))
      (`self.Check State`))))

(event `Check State`
  ;[1 1 1] Pawn Sense
  (switch `/Game/SkaGameAssets/Enemies/DarnBatAssets/BluePrints/E_AI_State` (`self.AI State`)
    (:`NewEnumerator1`
      (`self.Roam`))
    (:`NewEnumerator2`
      (`self.Chase Player` (stale `self.PawnSensing.OnSeePawn` Pawn)))
    (:`NewEnumerator3`
      (`self.Attack Player`))))

(event `self.PawnSensing.OnSeePawn`
  (params (Pawn :type "Pawn Object Reference"))
  ;[1 1 1] Pawn Sense
  (set `self.AI State` "NewEnumerator2")
  (`/Engine/EditorBlueprintResources/StandardMacros.DoOnce` false
    (:`Completed`
      (set `self.Is Down?` false)
      (`self.Check State`))))

(event `Attack Player`
  ;[1 1 1] Attack Player
  (`AnimInstance.Montage_Play` (`SkeletalMeshComponent.GetAnimInstance` (`self.Mesh`)) "/Game/SkaGameAssets/Enemies/Zombie_Anim_Zombie_Armature_Zombie_Attack_Montage.Zombie_Anim_Zombie_Armature_Zombie_Attack_Montage" 1.0 "MontageLength" 0.0)
  (`KismetSystemLibrary.Delay` 1.0)
  (set `self.AI State` "NewEnumerator2")
  (`self.Check State`))

(event `self.Sphere.OnComponentBeginOverlap`
  (params (OverlappedComponent :type "PrimitiveComponent Object Reference") (OtherActor :type "Actor Object Reference") (OtherComp :type "PrimitiveComponent Object Reference") (OtherBodyIndex :type Integer) (bFromSweep :type Boolean) (SweepResult :type "HitResult Structure (by ref)"))
  ;[1 1 1] Attack Player
  (`GameplayStatics.ApplyDamage` OtherActor 0.1))

(fn `Can Damage`
  (`PrimitiveComponent.SetCollisionEnabled` (`self.Sphere`) "QueryOnly"))

(fn `Cannot Damage`
  (`PrimitiveComponent.SetCollisionEnabled` (`self.Sphere`) "NoCollision"))

(fn `CheckDeath`
  (if (<= (`self.Health`) 0.0)
    (set `self.Is Down?` true)
    (`self.Wait`)))

(fn `UserConstructionScript`
  (`SceneComponent.K2_AttachToComponent` (`self.Sphere`) (`self.Mesh`) "Fingers_R" "KeepRelative" "KeepRelative" "KeepRelative" true))