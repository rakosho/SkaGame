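; GraveLord enemy Blueprint that reacts to any damage with a stun animation.
; AnyDamage calls Stun, which plays the hurt montage slightly slowed and waits on a Delay with nothing after it.
; The IsStunned resets are disconnected, so the event never changes that flag.
; The construction script attaches two capsules to the right and left palm sockets of the mesh.
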(event `Stun`
  ;[1 1 1] Stun
  (bind _returnvalue (`AnimInstance.Montage_Play` (`SkeletalMeshComponent.GetAnimInstance` (`self.Mesh`)) "/Game/SkaGameAssets/Enemies/RaveLordAssets/GraveLord__1__Anim_GraveLord_Armature_GraveLord_Hurt_Montage.GraveLord__1__Anim_GraveLord_Armature_GraveLord_Hurt_Montage" 0.8 "MontageLength" 0.0))
  (`KismetSystemLibrary.Delay` _returnvalue))

(event `self.ReceiveAnyDamage`
  (params (Damage :type "Float (single-precision)") (DamageType :type "DamageType Object Reference") (InstigatedBy :type "Controller Object Reference") (DamageCauser :type "Actor Object Reference"))
  (`self.Stun`))

(fn `UserConstructionScript`
  (bind _mesh (`self.Mesh`))
  (`SceneComponent.K2_AttachToComponent` (`self.Capsule`) _mesh "Palm_R" "KeepRelative" "KeepRelative" "KeepRelative" true)
  (`SceneComponent.K2_AttachToComponent` (`self.Capsule1`) _mesh "Palm_L" "KeepRelative" "KeepRelative" "KeepRelative" true))