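; Bat enemy character that roams random nearby navigable points and chases the side-scroller player when pawn sensing spots them.
; A simple Roam/Chase state drives AI move-to calls, with roaming looping and each chase returning to Roam when it ends.
; An attack sphere attached to the head socket damages overlapping actors while the attacking flag is set.
; Incoming damage lowers health and destroys the bat at zero.
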(event `self.ReceiveBeginPlay`
  ;[1 1 1] Initialize Bat
  (`PrimitiveComponent.IgnoreActorWhenMoving` (`self.AttackSphere`) null true)
  (set `self.AIState` "NewEnumerator1")
  (`self.CheckState`))

(event `CheckState`
  ;[1 1 1] Check the State of the AI
  (switch `/Game/SkaGameAssets/Enemies/DarnBatAssets/BluePrints/E_AI_State` "NewEnumerator1"
    (:`NewEnumerator1`
      (`self.Roam`))
    (:`NewEnumerator2`
      (`self.ChasePlayer` (`GameplayStatics.GetPlayerPawn` 0)))))

(event `Roam`
  ;[1 1 1] Roam
  (if (`|EnumEquality` (`self.AIState`) "NewEnumerator1")
    (`|AIMoveTo` self (`NavigationSystem.GetRandomPointInNavigableRadius` (`self.K2_GetActorLocation`) 500.0)
      (:`OnSuccess`
        _)
      (:`OnFail`
        _))
    (`self.CheckState`)))

(event `CheckDeath`
  ;[1 1 1] health/damage
  (if (<= (`self.Health`) 0.0)
    (`self.K2_DestroyActor`)))

(event `ChasePlayer`
  (params (PlayertoChase :type "Pawn Object Reference"))
  ;[1 1 1] ChasePlayer
  (if (not (`self.IsAttacking?`))
    (set `self.IsAttacking?` true)
    (`MovementComponent.StopMovementImmediately` (`self.CharacterMovement`)))
  (`|AIMoveTo` self (0.0 0.0 0.0) PlayertoChase 0.0
    (:`OnSuccess`
      (set `self.IsAttacking?` false)
      (`KismetSystemLibrary.Delay` 0.5))
    (:`OnFail`
      _))
  (set `self.AIState` "NewEnumerator1")
  (`self.CheckState`))

(event `self.ReceiveAnyDamage`
  (params (Damage :type "Float (single-precision)") (DamageType :type "DamageType Object Reference") (InstigatedBy :type "Controller Object Reference") (DamageCauser :type "Actor Object Reference"))
  ;[1 1 1] health/damage
  (set `self.Health` (- (`self.Health`) Damage))
  (`self.CheckDeath`))

(event `self.AttackSphere.OnComponentBeginOverlap`
  (params (OverlappedComponent :type "PrimitiveComponent Object Reference") (OtherActor :type "Actor Object Reference") (OtherComp :type "PrimitiveComponent Object Reference") (OtherBodyIndex :type Integer) (bFromSweep :type Boolean) (SweepResult :type "HitResult Structure (by ref)"))
  (if (`self.IsAttacking?`)
    (`GameplayStatics.ApplyDamage` OtherActor 0.2)))

(event `self.PawnSensing.OnSeePawn`
  (params (Pawn :type "Pawn Object Reference"))
  ;[1 1 1] chase player when we see the them
  (set `self.AIState` "NewEnumerator2")
  (bind _asside_scroller_character (cast `/Game/SkaGameAssets/Brad/Blueprints/SideScrollerCharacter` Pawn))
  (`self.ChasePlayer` _asside_scroller_character))

(fn `UserConstructionScript`
  (`SceneComponent.K2_AttachToComponent` (`self.AttackSphere`) (`self.Mesh`) "Head" "KeepRelative" "KeepRelative" "KeepRelative" true))