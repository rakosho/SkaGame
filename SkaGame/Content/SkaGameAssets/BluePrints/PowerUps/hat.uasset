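; Hat collectible for the side-scroller that spins by a fixed local rotation each tick.
; When the SideScrollerCharacter overlaps its mesh, it increments the character's Hats count, plays a sound at the world origin and destroys itself.
; When the count reaches exactly five, the character gains a life and the count resets to zero.
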(event `self.ReceiveTick`
  (params (DeltaSeconds :type "Float (single-precision)"))
  (`self.K2_AddActorLocalRotation` (struct :`Roll` 1.5)))

(event `self.StaticMesh.OnComponentBeginOverlap`
  (params (OverlappedComponent :type "PrimitiveComponent Object Reference") (OtherActor :type "Actor Object Reference") (OtherComp :type "PrimitiveComponent Object Reference") (OtherBodyIndex :type Integer) (bFromSweep :type Boolean) (SweepResult :type "HitResult Structure (by ref)"))
  (bind _asside_scroller_character (cast `/Game/SkaGameAssets/Brad/Blueprints/SideScrollerCharacter` OtherActor))
  (set `/Game/SkaGameAssets/Brad/Blueprints/SideScrollerCharacter.Hats` (+ (`/Game/SkaGameAssets/Brad/Blueprints/SideScrollerCharacter.Hats` _asside_scroller_character) 1.0) _asside_scroller_character)
  (`|ExecutionSequence`
    (:`then_0`
      (`/Engine/EditorBlueprintResources/StandardMacros.CompareFloat` (`/Game/SkaGameAssets/Brad/Blueprints/SideScrollerCharacter.Hats` _asside_scroller_character) 5.0
        (:`==`
          (if true
            (`|ExecutionSequence`
              (:`then_0`
                (set `/Game/SkaGameAssets/Brad/Blueprints/SideScrollerCharacter.Lives` (+ (`/Game/SkaGameAssets/Brad/Blueprints/SideScrollerCharacter.Lives` _asside_scroller_character) 1.0) _asside_scroller_character))
              (:`then_1`
                (set `/Game/SkaGameAssets/Brad/Blueprints/SideScrollerCharacter.Hats` (* (`/Game/SkaGameAssets/Brad/Blueprints/SideScrollerCharacter.Hats` _asside_scroller_character) 0.0) _asside_scroller_character)))))))
    (:`then_1`
      (`GameplayStatics.PlaySoundAtLocation` null)
      (`self.K2_DestroyActor`))))

(fn `UserConstructionScript`)