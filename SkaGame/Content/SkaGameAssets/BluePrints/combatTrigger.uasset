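; Combat trigger actor that springs a ghost encounter when something overlaps its collision component.
; After a short delay, it spawns three Ghost_BP pawns running GhostBehaviorTree at the positions of its three spawn location components.
; It then destroys itself, with no check on what caused the overlap.
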(event `self.CollisionComponent.OnComponentBeginOverlap`
  (params (OverlappedComponent :type "PrimitiveComponent Object Reference") (OtherActor :type "Actor Object Reference") (OtherComp :type "PrimitiveComponent Object Reference") (OtherBodyIndex :type Integer) (bFromSweep :type Boolean) (SweepResult :type "HitResult Structure (by ref)"))
  (`KismetSystemLibrary.Delay` 0.2)
  (`|ExecutionSequence`
    (:`then_0`
      (`AIBlueprintHelperLibrary.SpawnAIFromClass` "/Game/SkaGameAssets/BluePrints/Enemies/Ghost_BP.Ghost_BP_C" "/Game/SkaGameAssets/BluePrints/Enemies/AI/GhostBehaviorTree.GhostBehaviorTree" (`SceneComponent.GetSocketLocation` (`self.SpawnLocation`) "None"))
      (`AIBlueprintHelperLibrary.SpawnAIFromClass` "/Game/SkaGameAssets/BluePrints/Enemies/Ghost_BP.Ghost_BP_C" "/Game/SkaGameAssets/BluePrints/Enemies/AI/GhostBehaviorTree.GhostBehaviorTree" (`SceneComponent.GetSocketLocation` (`self.SpawnLocation2`) "None"))
      (`AIBlueprintHelperLibrary.SpawnAIFromClass` "/Game/SkaGameAssets/BluePrints/Enemies/Ghost_BP.Ghost_BP_C" "/Game/SkaGameAssets/BluePrints/Enemies/AI/GhostBehaviorTree.GhostBehaviorTree" (`SceneComponent.GetSocketLocation` (`self.SpawnLocation3`) "None")))
    (:`then_1`
      (`self.K2_DestroyActor`))))

(fn `UserConstructionScript`)